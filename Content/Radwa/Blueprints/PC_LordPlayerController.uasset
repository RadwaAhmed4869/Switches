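; Player controller for touch-controlled BP_Lord characters, handling tap selection and tap-to-move.
; On BeginPlay it adds the input mapping, shows the cursor and views through the lord's current camera volume.
; Touch press traces under the finger; release possesses a tapped lord and toggles its selection widget, or moves to the hit location.
; Re-tapping deselects without unpossessing, movement requires a minimum distance, and recorded screen touch positions go unused.
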(event Input|EnhancedActionEvents|EnhancedInputActionIA_SetDestination_Touch
  (params (ActionValue :type Boolean) (ElapsedSeconds :type Float%20%28double-precision%29) (TriggeredSeconds :type Float%20%28double-precision%29) (InputAction :type Input%20Action%20Object%20Reference :default "/Game/Radwa/Inputs/IA_SetDestination_Touch.IA_SetDestination_Touch"))
  (:Started
    (CallFunction|TouchPressed))
  (:Completed
    (CallFunction|TouchReleased)))

(event EventBeginPlay
  (bind _returnvalue (PlayerController|LocalPlayerSubsystems|GetEnhancedInputLocalPlayerSubsystem))
  (Utilities|IsValid _returnvalue
    (:Is%20Valid
      (Input|AddMappingContext _returnvalue "/Game/Radwa/Inputs/IMC_Character.IMC_Character" 0 "(bIgnoreAllPressedKeysUntilRelease=True,bForceImmediately=False)")
      (Variables|Default|SetbShowMouseCursor true)
      (bind _asbp_lord (Utilities|Casting|CastToBP_Lord (Game|Player|GetPlayerPawn 0)))
      (Utilities|IsValid (Variables|/Game/Radwa/Blueprints/Character/BP_Lord.BP_Lord_C|GetCurrentCameraVolume _asbp_lord)
        (:Is%20Valid
          (bind _output_get (Variables|Default|SetCurrentCamVol (Variables|/Game/Radwa/Blueprints/Character/BP_Lord.BP_Lord_C|GetCurrentCameraVolume _asbp_lord)))
          (Game|Player|SetViewTargetwithBlend _output_get 0.0 "VTBlend_Linear" 0.0 false))))))

(event EventTick
  (params (DeltaSeconds :type Float%20%28single-precision%29)))

(fn ConstructionScript)

(fn TouchPressed
  (bind (_locationx _locationy) (Class|PlayerController|GetInputTouchState "Touch1"))
  (bind _hitresult (Class|PlayerController|GetHitResultUnderFingerbyChannel "Touch1" "TraceTypeQuery1" true))
  (Variables|Default|SetInitTouchLocation (Math|Vector2D|MakeVector2D _locationx _locationy))
  (Variables|Default|SetHitResultLocation (.location _hitresult))
  (Variables|Default|SetHitActor (.hitactor _hitresult)))

(fn TouchReleased
  (bind (_locationx _locationy) (Class|PlayerController|GetInputTouchState "Touch1"))
  (Variables|Default|SetFinalTouchLocation (Math|Vector2D|MakeVector2D _locationx _locationy))
  (bind _asbp_lord (Utilities|Casting|CastToBP_Lord (Variables|Default|GetHitActor))
    (:then
      (Variables|Default|SetHitCharacter _asbp_lord)
      (Utilities|IsValid (Variables|Default|GetSelectedCharacter)
        (:Is%20Valid
          (Default|DisableSelectionWidget (Variables|Default|GetSelectedCharacter))
          (if (!= (Variables|Default|GetHitCharacter) (Variables|Default|GetSelectedCharacter))
            (Pawn|UnPossess)
            (CallFunction|Possessing)
            (else
              (Variables|Default|SetSelectedCharacter 0))))
        (:Is%20Not%20Valid
          (CallFunction|Possessing))))
    (:CastFailed
      (Utilities|IsValid (Variables|Default|GetSelectedCharacter)
        (:Is%20Valid
          (CallFunction|MovetoHitLocation (Variables|Default|GetHitResultLocation)))))))

(fn MovetoHitLocation
  (params (HitLocation :type Vector))
  (if (> (Math|Vector|VectorLength (- (Transformation|GetActorLocation (Game|Player|GetPlayerPawn 0)) (Variables|Default|GetHitResultLocation))) (Variables|Default|GetMinClickDistance))
    (AI|Navigation|SimpleMovetoLocation self HitLocation)))

(fn Possessing
  (bind _output_get (Variables|Default|SetSelectedCharacter (Variables|Default|GetHitCharacter)))
  (Default|EnableSelectionWidget _output_get)
  (Pawn|Possess _output_get))
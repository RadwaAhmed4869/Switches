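; BP_Wall is a switch-driven wall or door that either rises vertically or swings around its yaw axis, chosen by DoorType.
; It caches its starting transform on BeginPlay, and a timeline offsets the root from it on activation, with a sound.
; Deactivation reverses the timeline with the same sound, unless StayOpen is set, which instead sets AlreadyOpen so later activations are ignored.
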(event EventBeginPlay
  (Variables|Default|SetInitLocation (Transformation|GetActorLocation))
  (Variables|Default|SetInitRotation (Transformation|GetWorldRotation (Variables|Default|GetDefaultSceneRoot))))

(event EventOnSwitchActivated
  (bind _initlocation (Variables|Default|GetInitLocation))
  (bind _initrotation (Variables|Default|GetInitRotation))
  (if (not (Variables|Default|GetAlreadyOpen))
    (Audio|PlaySound2D (Variables|Default|GetSound) 0.6 1.0 0.0 0 0 false)
    (bind (_direction _doorelevation _doorrotatoin) (Timeline|DoorTimeline Play)
      (:Update
        (if (Utilities|Enum|Equal(Enum) (Variables|Default|GetDoorType) "NewEnumerator0")
          (Transformation|SetWorldLocation (Variables|Default|GetDefaultSceneRoot) (Math|Vector|MakeVector (.x _initlocation) (.y _initlocation) (+ (.z _initlocation) _doorelevation)) false false)
          (else
            (Transformation|SetWorldRotation (Variables|Default|GetDefaultSceneRoot) (Math|Rotator|MakeRotator (.roll _initrotation) (.pitch _initrotation) (+ (.yaw _initrotation) _doorrotatoin)) false false)))))))

(event EventOnSwitchDeactivated
  (bind _initlocation (Variables|Default|GetInitLocation))
  (bind _initrotation (Variables|Default|GetInitRotation))
  (if (Variables|Default|GetStayOpen)
    (Variables|Default|SetAlreadyOpen true)
    (else
      (Audio|PlaySound2D (Variables|Default|GetSound) 0.6 1.0 0.0 0 0 false)
      (bind (_direction _doorelevation _doorrotatoin) (Timeline|DoorTimeline Reverse)
        (:Update
          (if (Utilities|Enum|Equal(Enum) (Variables|Default|GetDoorType) "NewEnumerator0")
            (Transformation|SetWorldLocation (Variables|Default|GetDefaultSceneRoot) (Math|Vector|MakeVector (.x _initlocation) (.y _initlocation) (+ (.z _initlocation) _doorelevation)) false false)
            (else
              (Transformation|SetWorldRotation (Variables|Default|GetDefaultSceneRoot) (Math|Rotator|MakeRotator (.roll _initrotation) (.pitch _initrotation) (+ (.yaw _initrotation) _doorrotatoin)) false false))))))))

(fn ConstructionScript)
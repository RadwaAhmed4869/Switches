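; BP_Character is a character Blueprint that shows or hides an animated selection arrow to mark when it is selected.
; EnableSelectionWidget makes the SelectionArrow widget component visible and plays the arrow animation on its WBP_SelectionIcon widget.
; DisableSelectionWidget hides the component and stops that animation, and runs on BeginPlay so the character starts unselected.
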(event EventBeginPlay
  (CallFunction|DisableSelectionWidget))

(event Collision|EventActorBeginOverlap
  (params (OtherActor :type Actor%20Object%20Reference)))

(event EventTick
  (params (DeltaSeconds :type Float%20%28single-precision%29)))

(fn ConstructionScript)

(fn EnableSelectionWidget
  (bind _selectionarrow (Variables|Default|GetSelectionArrow))
  (bind _returnvalue (UserInterface|GetUserWidgetObject _selectionarrow))
  (Rendering|SetVisibility (Variables|Default|GetSelectionArrow) true true)
  (bind _aswbp_selection_icon (Utilities|Casting|CastToWBP_SelectionIcon _returnvalue))
  (UserInterface|Animation|PlayAnimation _returnvalue (Variables|/Game/Radwa/Blueprints/HUD/WBP_SelectionIcon.WBP_SelectionIcon_C|GetArrowAnimation _aswbp_selection_icon) 0.0 1 "Forward" 1.0 false))

(fn DisableSelectionWidget
  (bind _selectionarrow (Variables|Default|GetSelectionArrow))
  (bind _returnvalue (UserInterface|GetUserWidgetObject _selectionarrow))
  (Rendering|SetVisibility (Variables|Default|GetSelectionArrow) false true)
  (bind _aswbp_selection_icon (Utilities|Casting|CastToWBP_SelectionIcon _returnvalue))
  (Class|UserWidget|StopAnimation _returnvalue (Variables|/Game/Radwa/Blueprints/HUD/WBP_SelectionIcon.WBP_SelectionIcon_C|GetArrowAnimation _aswbp_selection_icon)))
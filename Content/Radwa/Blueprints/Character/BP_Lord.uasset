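; BP_Lord is a character Blueprint with a selection arrow indicator and a jump input.
; Enable and disable functions show or hide the SelectionArrow widget component and start or stop its WBP_SelectionIcon arrow animation, looping it while shown.
; BeginPlay hides the arrow, and the IA_Jump Enhanced Input action triggers Jump.
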(event Input|EnhancedActionEvents|EnhancedInputActionIA_Jump
  (params (ActionValue :type Boolean) (ElapsedSeconds :type Float%20%28double-precision%29) (TriggeredSeconds :type Float%20%28double-precision%29) (InputAction :type Input%20Action%20Object%20Reference :default "/Game/Radwa/Inputs/IA_Jump.IA_Jump"))
  (:Started
    (Character|Jump)))

(event EventBeginPlay
  (CallFunction|DisableSelectionWidget))

(event Collision|EventActorBeginOverlap
  (params (OtherActor :type Actor%20Object%20Reference)))

(event EventTick
  (params (DeltaSeconds :type Float%20%28single-precision%29)))

(fn ConstructionScript)

(fn EnableSelectionWidget
  (bind _selectionarrow (Variables|Default|GetSelectionArrow))
  (bind _returnvalue (UserInterface|GetUserWidgetObject _selectionarrow))
  (bind _aswbp_selection_icon (Utilities|Casting|CastToWBP_SelectionIcon _returnvalue))
  (UserInterface|Animation|PlayAnimation _returnvalue (Variables|/Game/Radwa/Blueprints/HUD/WBP_SelectionIcon.WBP_SelectionIcon_C|GetArrowAnimation _aswbp_selection_icon) 0.0 0 "Forward" 1.0 false)
  (Rendering|SetVisibility (Variables|Default|GetSelectionArrow) true false))

(fn DisableSelectionWidget
  (bind _selectionarrow (Variables|Default|GetSelectionArrow))
  (bind _returnvalue (UserInterface|GetUserWidgetObject _selectionarrow))
  (bind _aswbp_selection_icon (Utilities|Casting|CastToWBP_SelectionIcon _returnvalue))
  (Class|UserWidget|StopAnimation _returnvalue (Variables|/Game/Radwa/Blueprints/HUD/WBP_SelectionIcon.WBP_SelectionIcon_C|GetArrowAnimation _aswbp_selection_icon))
  (Rendering|SetVisibility (Variables|Default|GetSelectionArrow) false false))
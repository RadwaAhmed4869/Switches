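; BP_Switch is a pressure switch that BP_Gurad or BP_Lord actors trigger by overlapping its Box.
; It tracks occupants in RegisteredCharacters, so only the first to enter activates it and it deactivates when none remain.
; Each change sends an activated or deactivated message to every AffectedActors entry and plays a stone-grinding sound.
; SwitchTimeline offsets the switch's height from its starting location, playing on activation and reversing inside the deactivation loop.
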(event OnComponentBeginOverlap(Box)
  (params (OverlappedComponent :type Primitive%20Component%20Object%20Reference) (OtherActor :type Actor%20Object%20Reference) (OtherComp :type Primitive%20Component%20Object%20Reference) (OtherBodyIndex :type Integer) (bFromSweep :type Boolean) (SweepResult :type Hit%20Result%20Structure%20%28by%20ref%29))
  (bind _initlocation (Variables|Default|GetInitLocation))
  (bind _registeredcharacters (Variables|Default|GetRegisteredCharacters))
  (bind _asbp_gurad (Utilities|Casting|CastToBP_Gurad OtherActor)
    (:then
      _)
    (:CastFailed
      (Utilities|Casting|CastToBP_Lord OtherActor)))
  (Utilities|Array|Add _registeredcharacters _asbp_gurad)
  (if (== (Utilities|Array|Length _registeredcharacters) 1)
    (for _array_element (Variables|Default|GetAffectedActors)
      (Class|ISwitch|OnSwitchActivated(Message) _array_element))
    (Audio|PlaySound2D "/Game/Radwa/Sounds/StonesGrinding1_Cue.StonesGrinding1_Cue" 0.4 1.0 0.0 0 0 false)
    (bind _switchelevation (Timeline|SwitchTimeline Play)
      (:Update
        (Transformation|SetActorLocation (Math|Vector|MakeVector (.x _initlocation) (.y _initlocation) (+ (.z _initlocation) _switchelevation)) false false)))))

(event OnComponentEndOverlap(Box)
  (params (OverlappedComponent :type Primitive%20Component%20Object%20Reference) (OtherActor :type Actor%20Object%20Reference) (OtherComp :type Primitive%20Component%20Object%20Reference) (OtherBodyIndex :type Integer))
  (bind _initlocation (Variables|Default|GetInitLocation))
  (bind _registeredcharacters (Variables|Default|GetRegisteredCharacters))
  (bind _asbp_gurad (Utilities|Casting|CastToBP_Gurad OtherActor)
    (:then
      _)
    (:CastFailed
      (Utilities|Casting|CastToBP_Lord OtherActor)))
  (Utilities|Array|RemoveItem _registeredcharacters _asbp_gurad)
  (if (== (Utilities|Array|Length _registeredcharacters) 0)
    (for _array_element (Variables|Default|GetAffectedActors)
      (Class|ISwitch|OnSwitchDeactivated(Message) _array_element)
      (bind _switchelevation (Timeline|SwitchTimeline Reverse)
        (:Update
          (Transformation|SetActorLocation (Math|Vector|MakeVector (.x _initlocation) (.y _initlocation) (+ (.z _initlocation) _switchelevation)) false false))))
    (Audio|PlaySound2D "/Game/Radwa/Sounds/StonesGrinding1_Cue.StonesGrinding1_Cue" 0.4 1.0 0.0 0 0 false)))

(event EventBeginPlay
  (Variables|Default|SetInitLocation (Transformation|GetActorLocation)))

(event EventTick
  (params (DeltaSeconds :type Float%20%28single-precision%29)))

(fn ConstructionScript)
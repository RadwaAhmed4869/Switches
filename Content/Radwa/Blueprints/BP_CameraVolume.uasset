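; Camera trigger volume that takes over the player's view when BP_Lord enters its box.
; On overlap it registers itself as the current volume on the Lord and its player controller, then blends the view target to itself with ease-in-out.
; If spline use is enabled, Tick smoothly moves the camera to the spline point nearest the Lord and rotates it to look at them.
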(event OnComponentBeginOverlap(Box)
  (params (OverlappedComponent :type Primitive%20Component%20Object%20Reference) (OtherActor :type Actor%20Object%20Reference) (OtherComp :type Primitive%20Component%20Object%20Reference) (OtherBodyIndex :type Integer) (bFromSweep :type Boolean) (SweepResult :type Hit%20Result%20Structure%20%28by%20ref%29))
  (bind _asbp_lord (Utilities|Casting|CastToBP_Lord OtherActor))
  (bind _output_get (Variables|Default|SetLordRef _asbp_lord))
  (Variables|/Game/Radwa/Blueprints/Character/BP_Lord.BP_Lord_C|SetCurrentCameraVolume _output_get self)
  (Utilities|IsValid (Variables|Default|GetLordPlayerControllerRef)
    (:Is%20Valid
      (bind _output_get_2 (Variables|/Game/Radwa/Blueprints/PC_LordPlayerController.PC_LordPlayerController_C|SetCurrentCamVol (Variables|Default|GetLordPlayerControllerRef) self))
      (Game|Player|SetViewTargetwithBlend (Variables|Default|GetLordPlayerControllerRef) _output_get_2 2.0 "VTBlend_EaseInOut" 5.0 true))))

(event EventBeginPlay
  (bind _asbp_lord (Utilities|Casting|CastToBP_Lord (Game|Player|GetPlayerPawn 0)))
  (Variables|Default|SetLordRef _asbp_lord)
  (bind _aspc_lord_player_controller (Utilities|Casting|CastToPC_LordPlayerController (Game|GetPlayerController 0)))
  (Variables|Default|SetLordPlayerControllerRef _aspc_lord_player_controller)
  (Variables|Default|SetInitTransform (Transformation|GetWorldTransform (Variables|Default|GetCamera)))
  (Variables|Default|SetUseSpline (Variables|Default|GetEnableSpline)))

(event EventTick
  (params (DeltaSeconds :type Float%20%28single-precision%29))
  (Variables|Default|SetDelta%20Seconds DeltaSeconds)
  (if (Variables|Default|GetUseSpline)
    (Utilities|IsValid (Variables|Default|GetLordRef)
      (:Is%20Valid
        (Transformation|SetWorldLocationAndRotation (Variables|Default|GetCamera) (Math|Interpolation|VInterpTo (Transformation|GetWorldLocation (Variables|Default|GetCamera)) (Spline|FindLocationClosesttoWorldLocation (Variables|Default|GetSpline) (Transformation|GetActorLocation (Variables|Default|GetLordRef)) "World") (Variables|Default|GetDelta%20Seconds) 6.0) (Math|Interpolation|RInterpTo (Transformation|GetWorldRotation (Variables|Default|GetCamera)) (Math|Rotator|FindLookatRotation (Transformation|GetWorldLocation (Variables|Default|GetCamera)) (Transformation|GetActorLocation (Variables|Default|GetLordRef))) (Variables|Default|GetDelta%20Seconds) 6.0) false false)))))

(fn ConstructionScript)
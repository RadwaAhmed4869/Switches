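; BP_Floor is a floor actor that moves vertically in response to switch activations.
; It counts active switches and plays a timeline once the count reaches SwitchesRequired.
; The timeline's WallElevation track offsets the actor's Z from the location stored at BeginPlay.
; Any deactivation lowers the count and reverses the timeline unless StayOpen is set.
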(event EventBeginPlay
  (Variables|Default|SetInitLocation (Transformation|GetActorLocation)))

(event Collision|EventActorBeginOverlap
  (params (OtherActor :type Actor%20Object%20Reference)))

(event EventTick
  (params (DeltaSeconds :type Float%20%28single-precision%29)))

(event EventOnSwitchActivated
  (bind _initlocation (Variables|Default|GetInitLocation))
  (Math|Integer|IncrementInt (Variables|Default|GetSwitchedActivated)
    (:%20%20
      (if (>= (Variables|Default|GetSwitchedActivated) (Variables|Default|GetSwitchesRequired))
        (bind _wallelevation (Timeline|FloorTimeline Play)
          (:Update
            (Transformation|SetActorLocation (Math|Vector|MakeVector (.x _initlocation) (.y _initlocation) (+ (.z _initlocation) _wallelevation)) false false)))))))

(event EventOnSwitchDeactivated
  (bind _initlocation (Variables|Default|GetInitLocation))
  (Math|Integer|DecrementInt (Variables|Default|GetSwitchedActivated)
    (:%20%20
      (if (not (Variables|Default|GetStayOpen))
        (bind _wallelevation (Timeline|FloorTimeline Reverse)
          (:Update
            (Transformation|SetActorLocation (Math|Vector|MakeVector (.x _initlocation) (.y _initlocation) (+ (.z _initlocation) _wallelevation)) false false)))))))

(fn ConstructionScript)